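; Poo_BP is a dropping that acts as a finite nutrient source for nearby life.
; On BeginPlay it caches overlapping BiologicalMaster_BP actors from SphereOfInfluence and, if MyselliumConnected, registers them with the Mysellium_BP actor.
; A looping one-second timer feeds each cached actor, draining Nutrients per recipient and destroying itself when empty.
; With no life cached, Nutrients just decays toward zero without triggering destruction.
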(event `self.ReceiveBeginPlay`
  ;[1 1 1] BeginPlay - Create an array of Life nearby and set a timer to Provide Nutrients to Life each cycle
  (bind _returnvalue (`GameplayStatics.GetActorOfClass` "/Game/MyContent/Environment/Mysellium/Mysellium_BP.Mysellium_BP_C"))
  (set `self.Mysellium_Ref` _returnvalue)
  (set `self.Plants` (`PrimitiveComponent.GetOverlappingActors` (`self.SphereOfInfluence`) "/Game/MyContent/Environment/InteractableItems/Biological/BiologicalMaster_BP.BiologicalMaster_BP_C"))
  (`KismetSystemLibrary.K2_SetTimer` null "ProvideNutrientsToPlantsNearby" 1.0 true)
  (if (`self.MyselliumConnected`)
    (`self.ConnectPlantsToMysellium`)))

(event `ProvideNutrientsToPlantsNearby`
  ;[1 1 1] Provide Nutrients to Life nearby
  (if (!= (`KismetArrayLibrary.Array_Length` (`self.Plants`)) 0)
    (for _array_element (`self.Plants`)
      (bind _asbiological_master_bp (cast `/Game/MyContent/Environment/InteractableItems/Biological/BiologicalMaster_BP` _array_element))
      (`/Game/MyContent/Environment/InteractableItems/InteractableMaster_BP.ReceiveNutrients_Event` _asbiological_master_bp (`self.NutrientSupplyAmount`))
      (bind _output_get (set `self.Nutrients` (`KismetMathLibrary.FClamp` (- (`self.Nutrients`) (`self.NutrientSupplyAmount`)) 0.0 100.0)))
      (if (<= _output_get 0.0)
        (`self.K2_DestroyActor`)))
    (else
      (set `self.Nutrients` (`KismetMathLibrary.FClamp` (- (`self.Nutrients`) 1.0) 0.0 100.0)))))

(event `ConnectPlantsToMysellium`
  ;[1 1 1] Connect Plants to Mysellium
  (for _array_element (`self.Plants`)
    (bind _asbiological_master_bp (cast `/Game/MyContent/Environment/InteractableItems/Biological/BiologicalMaster_BP` _array_element))
    (`/Game/MyContent/Environment/Mysellium/Mysellium_BP.Add Life To Mysellium` (`self.Mysellium_Ref`) _asbiological_master_bp)))

(fn `UserConstructionScript`)