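; DropableMaster_BP is the base dropable item that links nearby level items, such as vegetation and rocks, to the mycelium trail.
; One second after BeginPlay, a one-shot timer gathers LevelItemMaster_BP actors overlapping its SphereOfInfluence and flags each as MycelliumConnected.
; A separate Illuminate event shows or hides its point light.
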(event `self.ReceiveBeginPlay`
  ;[1 1 1] Connect Vegetation and Rocks within proximity to the Mysellium Trail
  (`KismetSystemLibrary.K2_SetTimerDelegate` (delegate `UpdateLifeConnected`) 1.0))

(event `UpdateLifeConnected`
  ;[1 1 1] Connect Vegetation and Rocks within proximity to the Mysellium Trail
  (bind _output_get (set `self.ConnectedActors` (`PrimitiveComponent.GetOverlappingActors` (`self.SphereOfInfluence`) "/Game/MyContent/LevelItems/LevelItemMaster_BP.LevelItemMaster_BP_C")))
  (for _array_element _output_get
    (bind _aslevel_item_master_bp (cast `/Game/MyContent/LevelItems/LevelItemMaster_BP` _array_element))
    (set `/Game/MyContent/LevelItems/LevelItemMaster_BP.MycelliumConnected` true _aslevel_item_master_bp)))

(event `Illuminate`
  (params (IsOn :type Boolean))
  (bind _pointlight (`self.PointLight`))
  ;[1 1 1] Illuminate/Unilluminate
  (if IsOn
    (`SceneComponent.SetVisibility` _pointlight true false)
    (else
      (`SceneComponent.SetVisibility` _pointlight false false))))

(fn `UserConstructionScript`)