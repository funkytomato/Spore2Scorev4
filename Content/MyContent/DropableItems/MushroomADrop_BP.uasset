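; MushroomADrop_BP is a dropped mushroom item that the player picks up with the Interact input.
; When CanPickup is set, Interact or a custom event casts the player to Spore2ScoreCharacter and checks HasMushrooms.
; If true, it calls CallPickedUpMushroom with its mushroom type, destroys itself and plays a sound; otherwise it prints an inventory-full message.
; RotateToFacePlayer is an empty stub, and nothing in this graph sets CanPickup.
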(event `self.ReceiveBeginPlay`
  ;[1 1 1] BeginPlay - Get reference to Widget_BP
  (`parent.ReceiveBeginPlay`))

(event `InputAction|Interact`
  (params (Key :type "Key Structure"))
  ;[1 1 1] Interact with Mushroom
  (:`Pressed`
    (if (`self.CanPickup`) :!label _label
      (bind _asspore_2score_character (cast `/Game/MyContent/Characters/Blueprints/Spore2ScoreCharacter` (`GameplayStatics.GetPlayerCharacter` 0)))
      (if (`/Game/MyContent/Characters/Blueprints/Spore2ScoreCharacter.HasMushrooms` _asspore_2score_character)
        (`/Game/MyContent/Characters/Blueprints/Spore2ScoreCharacter.PickedUpMushroom` _asspore_2score_character "NewEnumerator0")
        (`self.K2_DestroyActor`)
        (`GameplayStatics.PlaySoundAtLocation` "/Game/MobileStarterContent/Audio/Explosion_Cue.Explosion_Cue" (`self.K2_GetActorLocation` _asspore_2score_character) (struct) 1.0 1.0 0.0 null null null)
        (else
          (`KismetSystemLibrary.PrintString` "Too many mushrooms within inventory"))))))

(event `CustomEvent`
  ;[1 1 1] Interact with Mushroom
  (goto _label))

(fn `RotateToFacePlayer`)

(fn `UserConstructionScript`
  (`parent.UserConstructionScript`))